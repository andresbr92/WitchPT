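; Gameplay ability that detaches the cauldron altar from the character carrying it.
; On activation it gets the altar from the avatar through MechanicsInterface, detaches it from the character and tells the character to remove its reference.
; It then removes active effects granting the cauldron carrying state tag and ends after a short delay.
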(event `self.K2_ActivateAbility`
  (bind _ascharacter (cast `Character` (`self.GetAvatarActorFromActorInfo`)))
  (if (`KismetSystemLibrary.DoesImplementInterface` _ascharacter "/Script/WitchPT.MechanicsInterface")
    (bind _returnvalue (message `MechanicsInterface.GetCauldronAltar` _ascharacter))
    (`CauldronAltar.DetachFromCharacter` _returnvalue _ascharacter)
    (message `MechanicsInterface.HandleRemoveCauldronAltar` _ascharacter)
    (`AbilitySystemComponent.RemoveActiveEffectsWithGrantedTags` (`AbilitySystemBlueprintLibrary.GetAbilitySystemComponent` (`self.GetAvatarActorFromActorInfo`)) (struct :`GameplayTags` (struct :`(TagName` "Character.State.Cauldron.Carrying"))))
    (`AbilityTask_WaitDelay.WaitDelay` 1.0
      (:`OnFinish`
        (`self.K2_EndAbility`)))))