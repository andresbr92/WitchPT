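; Gameplay ability that puts a character into cauldron placement mode and previews where the cauldron would go.
; On activation it gets the character's cauldron, starts its placement preview and applies the Placing gameplay effect through a MechanicsInterface check.
; A WaitForPlacementLocation task then feeds hit location and normal into the preview.
; The detach, Carrying-effect removal and delayed EndAbility chain is unwired, so this graph never ends the ability itself.
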(event `self.K2_ActivateAbility`
  (bind _ascharacter (cast `Character` (`self.GetAvatarActorFromActorInfo`)))
  (bind _returnvalue (message `MechanicsInterface.GetCauldronAltar` _ascharacter))
  (bind _output_get (set `self.Cauldron` _returnvalue))
  (`CauldronAltar.StartPlacementPreview` _output_get _ascharacter)
  (if (`KismetSystemLibrary.DoesImplementInterface` _ascharacter "/Script/WitchPT.MechanicsInterface")
    (`self.BP_ApplyGameplayEffectToOwner` "/Game/Blueprints/AbilitySystem/GameplayEffects/Cauldron/GE_Standard_Cauldron_Placing.GE_Standard_Cauldron_Placing_C")
    (`self.LookForPlacement`)))

(event `LookForPlacement`
  (bind (_asynctaskproxy _hitlocation _hitnormal) (`AT_WaitForPlacementLocation_SLT.WaitForPlacementLocation` 500.0)
    (:`OnLocationFound`
      (`CauldronAltar.UpdatePlacementPreview` (`self.Cauldron`) _hitlocation _hitnormal))))