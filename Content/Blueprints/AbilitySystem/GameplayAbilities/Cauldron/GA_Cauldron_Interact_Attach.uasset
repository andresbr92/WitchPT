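; Gameplay ability that attaches a player to a cauldron they interact with, triggered by a gameplay event carrying the cauldron and instigating character.
; It calls the cauldron's hold interaction with that character.
; If the character implements MechanicsInterface, it applies a carrying gameplay effect to the avatar and passes the cauldron to the character's altar message handler.
; The ability ends after a short delay, longer on the interface path.
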(event `self.K2_ActivateAbilityFromEvent`
  (params (EventData :type "GameplayEventData Structure (by ref)"))
  (bind (_eventtag _instigator _target) (break `GameplayEventData` EventData))
  (bind _asbp_cauldron (cast `/Game/Blueprints/Item/Cauldron/BP_Cauldron` _target))
  (set `self.As BP Cauldron` _asbp_cauldron)
  (bind _ascharacter (cast `Character` _instigator))
  (`CauldronAltar.OnHoldInteraction` (`self.As BP Cauldron`) _ascharacter)
  (if (`KismetSystemLibrary.DoesImplementInterface` _ascharacter "/Script/WitchPT.MechanicsInterface")
    (`AbilitySystemComponent.BP_ApplyGameplayEffectToSelf` :`self` (`AbilitySystemBlueprintLibrary.GetAbilitySystemComponent` (`self.GetAvatarActorFromActorInfo`)) :`GameplayEffectClass` "/Game/Blueprints/AbilitySystem/GameplayEffects/Cauldron/GE_Standard_Cauldron_Carrying.GE_Standard_Cauldron_Carrying_C" :`Level` (`KismetMathLibrary.Conv_IntToDouble` (`self.GetAbilityLevel`)))
    (message `MechanicsInterface.HandleSetCauldronAltar` _ascharacter (`self.As BP Cauldron`))
    (`AbilityTask_WaitDelay.WaitDelay` 1.0
      (:`OnFinish`
        (`self.K2_EndAbility`)))
    (else
      (`AbilityTask_WaitDelay.WaitDelay` 0.5
        (:`OnFinish`
          (`self.K2_EndAbility`))))))