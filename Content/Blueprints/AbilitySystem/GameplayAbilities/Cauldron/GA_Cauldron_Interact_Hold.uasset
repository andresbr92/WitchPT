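; Gameplay ability for the hold interaction on a cauldron, triggered by a gameplay event.
; It passes the instigating character to the target cauldron's hold-interaction handler, then applies the cauldron carrying gameplay effect to the avatar at ability level.
; The ability ends itself after a short fixed delay, with no explicit removal of the effect.
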(event `self.K2_ActivateAbilityFromEvent`
  (params (EventData :type "GameplayEventData Structure (by ref)"))
  (bind (_eventtag _instigator _target) (break `GameplayEventData` EventData))
  (`KismetSystemLibrary.PrintString` (`KismetSystemLibrary.GetObjectName` _instigator))
  (bind _asbp_cauldron (cast `/Game/Blueprints/Item/Cauldron/BP_Cauldron` _target))
  (bind _ascharacter (cast `Character` _instigator))
  (`CauldronAltar.OnHoldInteraction` _asbp_cauldron _ascharacter)
  (`AbilitySystemComponent.BP_ApplyGameplayEffectToSelf` :`self` (`AbilitySystemBlueprintLibrary.GetAbilitySystemComponent` (`self.GetAvatarActorFromActorInfo`)) :`GameplayEffectClass` "/Game/Blueprints/AbilitySystem/GameplayEffects/Cauldron/GE_Standard_Cauldron_Carrying.GE_Standard_Cauldron_Carrying_C" :`Level` (`KismetMathLibrary.Conv_IntToDouble` (`self.GetAbilityLevel`)))
  (`AbilityTask_WaitDelay.WaitDelay` 1.0
    (:`OnFinish`
      (`self.K2_EndAbility`))))