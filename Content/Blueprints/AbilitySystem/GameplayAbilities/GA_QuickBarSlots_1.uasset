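; Gameplay ability that selects the first quick bar slot.
; On activation it finds the WitchPTQuickBarComponent on the owning PlayerController and sets active slot index 0, then ends after a short delay.
; If the component is missing, the ability never calls EndAbility.
; Disconnected leftover nodes for triggering GA_Int_Interact and broadcasting a test async message never run.
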(event `self.K2_ActivateAbility`
  (bind _returnvalue (`Actor.GetComponentByClass` (`.PlayerController` (break `GameplayAbilityActorInfo` (`self.GetActorInfo`))) "/Script/WitchPT.WitchPTQuickBarComponent"))
  (`/Engine/EditorBlueprintResources/StandardMacros.IsValid` _returnvalue
    (:`Is Valid`
      (bind _output_get (set `self.QuickBarComponent` _returnvalue))
      (`WitchPTQuickBarComponent.SetActiveSlotIndex` _output_get 0)
      (`AbilityTask_WaitDelay.WaitDelay` 0.1
        (:`OnFinish`
          (`self.K2_EndAbility`))))))