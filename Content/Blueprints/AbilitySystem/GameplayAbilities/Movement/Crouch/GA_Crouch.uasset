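; GA_Crouch is a gameplay ability that makes the WitchPT character crouch for as long as the input is held.
; On activation it calls Crouch on the avatar and applies the GE_StandardCrouch effect, keeping the handle.
; A WaitInputRelease task ends the ability, which then removes that effect and calls UnCrouch.
; A leftover debug "Hello" print runs on every activation.
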(event `self.K2_ActivateAbility`
  (`KismetSystemLibrary.PrintString` "Hello")
  (bind _asbp_witch_ptcharacter (cast `/Game/Blueprints/Character/BP_WitchPTCharacter` (`self.GetAvatarActorFromActorInfo`)))
  (set `self.As BP Witch PTCharacter` _asbp_witch_ptcharacter)
  (`Character.Crouch` _asbp_witch_ptcharacter)
  (bind _returnvalue (`self.BP_ApplyGameplayEffectToOwner` "/Game/Blueprints/AbilitySystem/GameplayAbilities/Movement/Crouch/GE_StandardCrouch.GE_StandardCrouch_C"))
  (set `self.CrouchEffectHandle` _returnvalue)
  (`AbilityTask_WaitInputRelease.WaitInputRelease` true
    (:`OnRelease`
      (`self.K2_EndAbility`))))

(event `self.K2_OnEndAbility`
  (params (bWasCancelled :type Boolean))
  (`self.BP_RemoveGameplayEffectFromOwnerWithHandle` (`self.CrouchEffectHandle`))
  (`Character.UnCrouch` (`self.As BP Witch PTCharacter`)))