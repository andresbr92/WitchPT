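; Gameplay ability for a player occupying a ritual altar position, triggered by an event whose target implements MechanicsInterface.
; It applies in-position and blocked effects to the owner, then tells the position the player has occupied it.
; Gameplay event waits forward four directional ritual inputs and the start request to the position.
; When the altar's interaction-completed delegate fires, it removes both effects and ends, regardless of success.
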(event `self.K2_ActivateAbilityFromEvent`
  (params (EventData :type "GameplayEventData Structure (by ref)"))
  (bind (_eventtag _instigator _target) (break `GameplayEventData` EventData))
  (if (`KismetSystemLibrary.DoesImplementInterface` _target "/Script/WitchPT.MechanicsInterface")
    (bind _returnvalue (`AbilitySystemComponent.BP_ApplyGameplayEffectToSelf` :`self` (`self.GetAbilitySystemComponentFromActorInfo`) :`GameplayEffectClass` "/Game/Blueprints/AbilitySystem/GameplayEffects/Ritual/GE_StandardRitualInPosition.GE_StandardRitualInPosition_C"))
    (set `self.GE_ParticipatingInAltar` _returnvalue)
    (bind _returnvalue_2 (`AbilitySystemComponent.BP_ApplyGameplayEffectToSelf` :`self` (`self.GetAbilitySystemComponentFromActorInfo`) :`GameplayEffectClass` "/Game/Blueprints/AbilitySystem/GameplayEffects/Ritual/GE_StandardBlocked.GE_StandardBlocked_C"))
    (set `self.GE_Blocked` _returnvalue_2)
    (set `self.RitualPosition` _target)
    (bind _ascharacter (cast `Character` _instigator))
    (set `self.As Character` _ascharacter)
    (`|ExecutionSequence`
      (:`then_0`
        ; Wait Ritual Inputs
        (message `MechanicsInterface.SendPlayerOccupiedPosition` (`self.RitualPosition`) (`self.As Character`))
        (bind (_asynctaskproxy _payload) (`AbilityTask_WaitGameplayEvent.WaitGameplayEvent` (struct :`TagName` "Ritual.Input.Down") null)
          (:`EventReceived`
            (message `MechanicsInterface.SendPlayerInput` (`self.RitualPosition`) (`self.As Character`) (`.EventTag` (break `GameplayEventData` _payload))))))
      (:`then_1`
        (bind (_asynctaskproxy_2 _payload_2) (`AbilityTask_WaitGameplayEvent.WaitGameplayEvent` (struct :`TagName` "Ritual.Input.Left") null)
          (:`EventReceived`
            (message `MechanicsInterface.SendPlayerInput` (`self.RitualPosition`) (`self.As Character`) (`.EventTag` (break `GameplayEventData` _payload_2))))))
      (:`then_2`
        (bind (_asynctaskproxy_3 _payload_3) (`AbilityTask_WaitGameplayEvent.WaitGameplayEvent` (struct :`TagName` "Ritual.Input.Right") null)
          (:`EventReceived`
            (message `MechanicsInterface.SendPlayerInput` (`self.RitualPosition`) (`self.As Character`) (`.EventTag` (break `GameplayEventData` _payload_3))))))
      (:`then_3`
        (bind (_asynctaskproxy_4 _payload_4) (`AbilityTask_WaitGameplayEvent.WaitGameplayEvent` (struct :`TagName` "Ritual.Input.Up") null)
          (:`EventReceived`
            (message `MechanicsInterface.SendPlayerInput` (`self.RitualPosition`) (`self.As Character`) (`.EventTag` (break `GameplayEventData` _payload_4))))))
      (:`then_4`
        ; Ritual Start
        (bind (_asynctaskproxy_5 _payload_5) (`AbilityTask_WaitGameplayEvent.WaitGameplayEvent` (struct :`TagName` "Ability.Altar.Start") null)
          (:`EventReceived`
            (message `MechanicsInterface.SendStartRitualRequest` (`self.RitualPosition`) (`self.As Character`)))))
      (:`then_5`
        ; Comment
        (bind _returnvalue_3 (message `MechanicsInterface.GetRitualAltarActor` (`self.RitualPosition`)))
        (add `BaseInteractableAltar.OnInteractionCompleted` _returnvalue_3 (delegate `OnInteractionCompleted_Event`))))
    (else
      (`self.K2_EndAbility`))))

(event `OnInteractionCompleted_Event`
  (params (bWasSuccessful :type Boolean))
  ; Comment
  (`AbilitySystemComponent.RemoveActiveGameplayEffect` (`self.GetAbilitySystemComponentFromActorInfo`) (`self.GE_Blocked`) -1)
  (`AbilitySystemComponent.RemoveActiveGameplayEffect` (`self.GetAbilitySystemComponentFromActorInfo`) (`self.GE_ParticipatingInAltar`) -1)
  (`self.K2_EndAbility`))