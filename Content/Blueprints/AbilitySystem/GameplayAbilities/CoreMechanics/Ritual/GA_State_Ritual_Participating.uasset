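; Gameplay ability that runs while a character occupies a position at a ritual altar, triggered by an event targeting that position.
; It opens the ritual view for the local player, feeds the altar to its view model, and applies in-position and blocked effects.
; Gameplay events for start, directional inputs and cancel are forwarded as requests through the character's mechanics interface.
; Completion removes the effects; cancel also frees the position, and locally closes the UI and ends the ability.
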(event `self.K2_ActivateAbilityFromEvent`
  (params (EventData :type "GameplayEventData Structure (by ref)"))
  (bind (_eventtag _instigator _target) (break `GameplayEventData` EventData))
  (bind _output_get (set `self.RitualPosition` _target))
  (if (`KismetSystemLibrary.DoesImplementInterface` _output_get "/Script/WitchPT.PositionInterface")
    (bind _returnvalue (message `PositionInterface.GetRitualAltarActor` (`self.RitualPosition`)))
    (bind _output_get_2 (set `self.RitualAltar` _returnvalue))
    (`/Engine/EditorBlueprintResources/StandardMacros.IsValid` _output_get_2
      (:`Is Valid`
        (`|ExecutionSequence`
          (:`then_0`
            (`self.IsLocallyControlled`
              (:`True`
                (`|ExecutionSequence`
                  (:`then_0`
                    (bind _returnvalue_2 (`UI_ManagerSubsystem.PushContentToLayer_ForPlayer` (subsystem `UI_ManagerSubsystem`) (`GameplayStatics.GetPlayerController` 0) (struct :`TagName` "UI.Layer.GameMenu") "/Game/Blueprints/UI/Ritual/WBP_RitualView.WBP_RitualView_C"))
                    (`UI_ManagerSubsystem.FocusModal` (subsystem `UI_ManagerSubsystem`) (`GameplayStatics.GetPlayerController` 0) _returnvalue_2 true false))
                  (:`then_1`
                    (bind _asmvvm_ritual_view_model (cast `MVVM_RitualViewModel` (`MVVMViewModelCollectionObject.FindViewModelInstance` (`MVVMGameSubsystem.GetViewModelCollection` (subsystem `MVVMGameSubsystem`)) (`self.Context`))))
                    (`MVVM_RitualViewModel.SetRitualAltar` _asmvvm_ritual_view_model (`self.RitualAltar`)))))))
          (:`then_1`
            (bind _ascharacter (cast `Character` _instigator))
            (set `self.As Character` _ascharacter)
            (if (`KismetSystemLibrary.IsValidInterface` (`WitchPTAbilitySystemLibrary.GetMechanicsInterface` (`self.As Character`)))
              (bind _returnvalue_3 (`AbilitySystemComponent.BP_ApplyGameplayEffectToSelf` :`self` (`self.GetAbilitySystemComponentFromActorInfo`) :`GameplayEffectClass` "/Game/Blueprints/AbilitySystem/GameplayEffects/Ritual/GE_StandardRitualInPosition.GE_StandardRitualInPosition_C"))
              (set `self.GE_ParticipatingInAltar` _returnvalue_3)
              (bind _returnvalue_4 (`AbilitySystemComponent.BP_ApplyGameplayEffectToSelf` :`self` (`self.GetAbilitySystemComponentFromActorInfo`) :`GameplayEffectClass` "/Game/Blueprints/AbilitySystem/GameplayEffects/Ritual/GE_StandardBlocked.GE_StandardBlocked_C"))
              (set `self.GE_Blocked` _returnvalue_4)
              ; Wait Ritual Inputs
              (`|ExecutionSequence`
                (:`then_0`
                  (bind (_asynctaskproxy _payload) (`AbilityTask_WaitGameplayEvent.WaitGameplayEvent` (struct :`TagName` "Ability.Ritual.Start") null)
                    (:`EventReceived`
                      (`MechanicsInterface.RequestStartRitual` (`WitchPTAbilitySystemLibrary.GetMechanicsInterface` (`self.As Character`)) (`self.RitualAltar`)))))
                (:`then_1`
                  (bind (_asynctaskproxy_2 _payload_2) (`AbilityTask_WaitGameplayEvent.WaitGameplayEvent` (struct :`TagName` "Ritual.Input.Up") null)
                    (:`EventReceived`
                      (`MechanicsInterface.RequestRitualInput` (`WitchPTAbilitySystemLibrary.GetMechanicsInterface` (`self.As Character`)) (`self.RitualAltar`) (`.EventTag` (break `GameplayEventData` _payload_2))))))
                (:`then_2`
                  (bind (_asynctaskproxy_3 _payload_3) (`AbilityTask_WaitGameplayEvent.WaitGameplayEvent` (struct :`TagName` "Ritual.Input.Down") null)
                    (:`EventReceived`
                      (`MechanicsInterface.RequestRitualInput` (`WitchPTAbilitySystemLibrary.GetMechanicsInterface` (`self.As Character`)) (`self.RitualAltar`) (`.EventTag` (break `GameplayEventData` _payload_3))))))
                (:`then_3`
                  (bind (_asynctaskproxy_4 _payload_4) (`AbilityTask_WaitGameplayEvent.WaitGameplayEvent` (struct :`TagName` "Ritual.Input.Right") null)
                    (:`EventReceived`
                      (`MechanicsInterface.RequestRitualInput` (`WitchPTAbilitySystemLibrary.GetMechanicsInterface` (`self.As Character`)) (`self.RitualAltar`) (`.EventTag` (break `GameplayEventData` _payload_4))))))
                (:`then_4`
                  (bind (_asynctaskproxy_5 _payload_5) (`AbilityTask_WaitGameplayEvent.WaitGameplayEvent` (struct :`TagName` "Ritual.Input.Left") null)
                    (:`EventReceived`
                      (`MechanicsInterface.RequestRitualInput` (`WitchPTAbilitySystemLibrary.GetMechanicsInterface` (`self.As Character`)) (`self.RitualAltar`) (`.EventTag` (break `GameplayEventData` _payload_5))))))
                (:`then_5`
                  (add `RitualAltar.OnRitualCompletedEvent` (`self.RitualAltar`) (delegate `OnRitualCompletedEvent_Event`)))
                (:`then_6`
                  (`AbilityTask_WaitGameplayEvent.WaitGameplayEvent` (struct :`TagName` "Ability.Ritual.CancelParticipatingInRitual") null
                    (:`EventReceived`
                      (bind _asbase_interaction_position (cast `BaseInteractionPosition` (`self.RitualPosition`)))
                      (`MechanicsInterface.RequestUnOccupyPositionInRitual` (`WitchPTAbilitySystemLibrary.GetMechanicsInterface` (`self.As Character`)) (`self.RitualAltar`) _asbase_interaction_position)
                      (`AbilitySystemComponent.RemoveActiveGameplayEffect` (`self.GetAbilitySystemComponentFromActorInfo`) (`self.GE_Blocked`) -1)
                      (`AbilitySystemComponent.RemoveActiveGameplayEffect` (`self.GetAbilitySystemComponentFromActorInfo`) (`self.GE_ParticipatingInAltar`) -1)
                      (`self.IsLocallyControlled`
                        (:`True`
                          (`UI_ManagerSubsystem.PopContentFromLayer_ForPlayer` (subsystem `UI_ManagerSubsystem`) (`GameplayStatics.GetPlayerController` 0) (struct :`TagName` "UI.Layer.GameMenu") -1)
                          (`UI_ManagerSubsystem.FocusGame` (subsystem `UI_ManagerSubsystem`) (`GameplayStatics.GetPlayerController` 0))
                          (`self.K2_EndAbility`)))))))
              (else
                (`self.K2_EndAbility`)))))))))

(event `OnRitualCompletedEvent_Event`
  (params (bWasSuccessful :type Boolean))
  (`AbilitySystemComponent.RemoveActiveGameplayEffect` (`self.GetAbilitySystemComponentFromActorInfo`) (`self.GE_Blocked`) -1)
  (`AbilitySystemComponent.RemoveActiveGameplayEffect` (`self.GetAbilitySystemComponentFromActorInfo`) (`self.GE_ParticipatingInAltar`) -1))