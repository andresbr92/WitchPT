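; Gameplay ability, triggered by event, that moves a character onto a ritual position to participate at an altar.
; If the target implements MechanicsInterface, it moves the avatar to that XY, keeping its height, under a temporary movement effect.
; On arrival it applies blocked and occupying effects, grants input success/failure abilities and sends the Participating event.
; The effect cleanup is unwired, so the ability ends only for invalid targets.
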(event `self.K2_ActivateAbility`)

(event `self.K2_ActivateAbilityFromEvent`
  (params (EventData :type "GameplayEventData Structure (by ref)"))
  (bind (_returnvalue_x _returnvalue_y) (`KismetMathLibrary.BreakVector` (`Actor.K2_GetActorLocation` EventData_Target)))
  (bind (_returnvalue_x_2 _returnvalue_y_2 _returnvalue_z) (`KismetMathLibrary.BreakVector` (`Actor.K2_GetActorLocation` (`self.GetAvatarActorFromActorInfo`))))
  (if (`KismetSystemLibrary.DoesImplementInterface` EventData_Target "/Script/WitchPT.MechanicsInterface")
    (bind _returnvalue (`AbilitySystemComponent.BP_ApplyGameplayEffectToSelf` :`self` (`self.GetAbilitySystemComponentFromActorInfo`) :`GameplayEffectClass` "/Game/Blueprints/AbilitySystem/GameplayEffects/Ritual/GE_StarndardMoveToRitualPosition.GE_StarndardMoveToRitualPosition_C" :`Level` (`KismetMathLibrary.Conv_IntToDouble` (`self.GetAbilityLevel`))))
    (`AbilityTask_MoveToLocation.MoveToLocation` "None" (`KismetMathLibrary.MakeVector` _returnvalue_x _returnvalue_y _returnvalue_z) 1.0
      (:`OnTargetLocationReached`
        (`self.BP_RemoveGameplayEffectFromOwnerWithHandle` _returnvalue)
        (bind _returnvalue_2 (`AbilitySystemComponent.BP_ApplyGameplayEffectToSelf` (`self.GetAbilitySystemComponentFromActorInfo`) "/Game/Blueprints/AbilitySystem/GameplayEffects/Ritual/GE_StandardBlocked.GE_StandardBlocked_C" (`KismetMathLibrary.Conv_IntToDouble` (`self.GetAbilityLevel`)) (make `GameplayEffectContextHandle`)))
        (set `self.GE_Blocked` _returnvalue_2)
        (bind _returnvalue_3 (`AbilitySystemComponent.BP_ApplyGameplayEffectToSelf` (`self.GetAbilitySystemComponentFromActorInfo`) "/Game/Blueprints/AbilitySystem/GameplayEffects/Ritual/GE_Ritual_OccupyingPosition.GE_Ritual_OccupyingPosition_C" (`KismetMathLibrary.Conv_IntToDouble` (`self.GetAbilityLevel`)) (make `GameplayEffectContextHandle`)))
        (set `self.GE_OccupyingPosition` _returnvalue_3)
        (`AbilitySystemComponent.K2_GiveAbility` (`self.GetAbilitySystemComponentFromActorInfo`) "/Game/Blueprints/AbilitySystem/GameplayAbilities/CoreMechanics/Ritual/Input/GA_Input_Failure.GA_Input_Failure_C" 1 -1)
        (`AbilitySystemComponent.K2_GiveAbility` (`self.GetAbilitySystemComponentFromActorInfo`) "/Game/Blueprints/AbilitySystem/GameplayAbilities/CoreMechanics/Ritual/Input/GA_Input_Success.GA_Input_Success_C" 1 -1)
        (`self.SendGameplayEvent` (struct :`TagName` "Ability.Altar.Participating") (make `GameplayEventData` (struct) EventData_Instigator EventData_Target))))
    (else
      (`self.K2_EndAbility`))))

(fn `GetRitualPositionObject`
  (params (Object :type "Object Object Reference"))
  (cast `/Game/Blueprints/Item/Ritual/BP_Ritual_Position` Object))