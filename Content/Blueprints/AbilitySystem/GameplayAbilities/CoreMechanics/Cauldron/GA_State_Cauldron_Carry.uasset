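; Gameplay ability for the cauldron carry state, from pickup request through placement preview to setting it down.
; On event activation it messages the target through MechanicsInterface, applies a carrying effect and listens for three gameplay events.
; Looking-for-place adds a placing effect and runs a WaitForPlacementLocation task that feeds hit location and normal to the preview.
; Cancel clears only placing state, while set-in-place finalizes placement, removes both effects and ends the ability.
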(event `self.K2_ActivateAbilityFromEvent`
  (params (EventData :type "GameplayEventData Structure (by ref)"))
  (bind (_eventtag _instigator _target) (break `GameplayEventData` EventData))
  (if (`KismetSystemLibrary.DoesImplementInterface` _target "/Script/WitchPT.MechanicsInterface")
    (bind _ascharacter (cast `Character` _instigator))
    (message `MechanicsInterface.SendStartCarryCauldronRequest` _target _ascharacter)
    (bind _returnvalue (`AbilitySystemComponent.BP_ApplyGameplayEffectToSelf` :`self` (`AbilitySystemBlueprintLibrary.GetAbilitySystemComponent` (`self.GetAvatarActorFromActorInfo`)) :`GameplayEffectClass` "/Game/Blueprints/AbilitySystem/GameplayEffects/Cauldron/GE_Standard_Cauldron_Carrying.GE_Standard_Cauldron_Carrying_C" :`Level` (`KismetMathLibrary.Conv_IntToDouble` (`self.GetAbilityLevel`))))
    (set `self.GE_Carrying` _returnvalue)
    (`|ExecutionSequence`
      (:`then_0`
        (`AbilityTask_WaitGameplayEvent.WaitGameplayEvent` (struct :`TagName` "Ability.Cauldron.LookingForPlaceCauldron") null false false
          (:`EventReceived`
            (bind _returnvalue_2 (`self.BP_ApplyGameplayEffectToOwner` "/Game/Blueprints/AbilitySystem/GameplayEffects/Cauldron/GE_Standard_Cauldron_Placing.GE_Standard_Cauldron_Placing_C"))
            (set `self.GE_Placing` _returnvalue_2)
            (message `MechanicsInterface.SendStartPlacementPreview` _target _ascharacter)
            (bind (_asynctaskproxy _hitlocation _hitnormal) (`AT_WaitForPlacementLocation_SLT.WaitForPlacementLocation` 500.0)
              (:`then`
                (set `self.WaitForPlacementTask` _asynctaskproxy))
              (:`OnLocationFound`
                (message `MechanicsInterface.SendUpdatePlacementPreview` _target _hitlocation _hitnormal))))))
      (:`then_1`
        (`AbilityTask_WaitGameplayEvent.WaitGameplayEvent` (struct :`TagName` "Ability.Cauldron.SetInPlace") null
          (:`EventReceived`
            (message `MechanicsInterface.SendFinalizePlacement` _target)
            (`GameplayTask.EndTask` (`self.WaitForPlacementTask`))
            (`self.BP_RemoveGameplayEffectFromOwnerWithHandle` (`self.GE_Placing`))
            (`self.BP_RemoveGameplayEffectFromOwnerWithHandle` (`self.GE_Carrying`))
            (`self.K2_EndAbility`))))
      (:`then_2`
        (`AbilityTask_WaitGameplayEvent.WaitGameplayEvent` (struct :`TagName` "Ability.Cauldron.CancelSetInPlace") null
          (:`EventReceived`
            (message `MechanicsInterface.SendCancelPlacementPreview` _target)
            (`self.BP_RemoveGameplayEffectFromOwnerWithHandle` (`self.GE_Placing`))
            (`GameplayTask.EndTask` (`self.WaitForPlacementTask`))))))))