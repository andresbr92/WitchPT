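; Event-activated gameplay ability that lets a character carry and place a cauldron.
; Asks the target to start carrying via MechanicsInterface messages and applies a carrying effect.
; Parallel gameplay event waits handle placement: searching applies a placing effect and feeds WaitForPlacementLocation hits into the target's preview.
; Confirming finalizes placement and ends the ability; cancelling stops the preview and location task but leaves the ability active.
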(event `self.K2_ActivateAbilityFromEvent`
  (params (EventData :type "GameplayEventData Structure (by ref)"))
  (bind (_eventtag _instigator _target) (break `GameplayEventData` EventData))
  (if (`KismetSystemLibrary.DoesImplementInterface` _target "/Script/WitchPT.MechanicsInterface")
    (bind _ascharacter (cast `Character` _instigator))
    (message `MechanicsInterface.SendStartCarryCauldronRequest` _target _ascharacter)
    (`AbilitySystemComponent.BP_ApplyGameplayEffectToSelf` :`self` (`AbilitySystemBlueprintLibrary.GetAbilitySystemComponent` (`self.GetAvatarActorFromActorInfo`)) :`GameplayEffectClass` "/Game/Blueprints/AbilitySystem/GameplayEffects/Cauldron/GE_Standard_Cauldron_Carrying.GE_Standard_Cauldron_Carrying_C" :`Level` (`KismetMathLibrary.Conv_IntToDouble` (`self.GetAbilityLevel`)))
    (`|ExecutionSequence`
      (:`then_0`
        (`AbilityTask_WaitGameplayEvent.WaitGameplayEvent` (struct :`TagName` "Ability.Cauldron.LookingForPlaceCauldron") null
          (:`EventReceived`
            (`self.BP_ApplyGameplayEffectToOwner` "/Game/Blueprints/AbilitySystem/GameplayEffects/Cauldron/GE_Standard_Cauldron_Placing.GE_Standard_Cauldron_Placing_C")
            (message `MechanicsInterface.SendStartPlacementPreview` _target _ascharacter)
            (bind (_asynctaskproxy _hitlocation _hitnormal) (`AT_WaitForPlacementLocation_SLT.WaitForPlacementLocation` 500.0 10.0 false false true)
              (:`then`
                (set `self.WaitForPlacementTask` _asynctaskproxy))
              (:`OnLocationFound`
                (message `MechanicsInterface.SendUpdatePlacementPreview` _target _hitlocation _hitnormal))))))
      (:`then_1`
        (`AbilityTask_WaitGameplayEvent.WaitGameplayEvent` (struct :`TagName` "Ability.Cauldron.SetInPlace") null
          (:`EventReceived`
            (message `MechanicsInterface.SendFinalizePlacement` _target)
            (`GameplayTask.EndTask` (`self.WaitForPlacementTask`))
            (`self.K2_EndAbility`))))
      (:`then_2`
        (`AbilityTask_WaitGameplayEvent.WaitGameplayEvent` (struct :`TagName` "Ability.Cauldron.CancelSetInPlace") null
          (:`EventReceived`
            (message `MechanicsInterface.SendCancelPlacementPreview` _target)
            (`GameplayTask.EndTask` (`self.WaitForPlacementTask`))))))))