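; Gameplay ability that moves a witch character onto a ritual position and claims it, triggered by a gameplay event carrying the position and instigator.
; It ends if the position is occupied, otherwise slides the character there at its current height under a temporary movement effect.
; On arrival it applies blocked and occupying effects, marks the position occupied, records it on the player state and ends.
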(event `self.K2_ActivateAbility`)

(event `self.K2_ActivateAbilityFromEvent`
  (params (EventData :type "GameplayEventData Structure (by ref)"))
  (bind (_returnvalue_x _returnvalue_y _returnvalue_z) (`KismetMathLibrary.BreakVector` (`Actor.K2_GetActorLocation` EventData_Instigator)))
  (bind _as_ritual_position (`self.As Ritual Position`))
  (bind (_returnvalue_x_2 _returnvalue_y_2) (`KismetMathLibrary.BreakVector` (`Actor.K2_GetActorLocation` (`self.As Ritual Position`))))
  (`|ExecutionSequence`
    (:`then_0`
      (`self.GetRitualPositionObject` EventData_Target)
      (bind _returnvalue (`self.CheckIsOccupied`))
      (if _returnvalue
        (`self.K2_EndAbility`)
        (else
          (set `self.RitualAltar` (`RitualPosition.GetRitualAltar` (`self.As Ritual Position`)))
          (bind _output_get (`self.GetCharacter` EventData_Instigator))
          (bind _returnvalue_2 (`AbilitySystemBlueprintLibrary.GetAbilitySystemComponent` _output_get))
          (bind _returnvalue_3 (`AbilitySystemComponent.BP_ApplyGameplayEffectToSelf` :`self` _returnvalue_2 :`GameplayEffectClass` "/Game/Blueprints/AbilitySystem/GameplayEffects/Ritual/GE_StarndardMoveToRitualPosition.GE_StarndardMoveToRitualPosition_C" :`Level` (`KismetMathLibrary.Conv_IntToDouble` (`self.GetAbilityLevel`))))
          (`AbilityTask_MoveToLocation.MoveToLocation` "None" (`KismetMathLibrary.MakeVector` _returnvalue_x_2 _returnvalue_y_2 _returnvalue_z) 1.0
            (:`OnTargetLocationReached`
              (`self.BP_RemoveGameplayEffectFromOwnerWithHandle` _returnvalue_3)
              (bind _returnvalue_4 (`AbilitySystemComponent.BP_ApplyGameplayEffectToSelf` :`self` _returnvalue_2 :`GameplayEffectClass` "/Game/Blueprints/AbilitySystem/GameplayEffects/Ritual/GE_StandardBlocked.GE_StandardBlocked_C" :`Level` (`KismetMathLibrary.Conv_IntToDouble` (`self.GetAbilityLevel`))))
              (set `self.GE_Blocked` _returnvalue_4)
              (`RitualPosition.SetOccupied` _as_ritual_position (`self.As BP Witch PTCharacter`))
              (`AbilitySystemComponent.BP_ApplyGameplayEffectToSelf` :`self` _returnvalue_2 :`GameplayEffectClass` "/Game/Blueprints/AbilitySystem/GameplayEffects/Ritual/GE_Ritual_OccupyingPosition.GE_Ritual_OccupyingPosition_C" :`Level` 1.0)
              (bind _asbp_witch_ptplayer_state (cast `/Game/Blueprints/Player/BP_WitchPTPlayerState` (`Pawn.PlayerState` (`self.As BP Witch PTCharacter`))))
              (`WitchPTPlayerState.SetRitualAltarInteractingWith` _asbp_witch_ptplayer_state (`self.As Ritual Position`))
              (`self.K2_EndAbility`)
              (`KismetSystemLibrary.PrintString` (`KismetSystemLibrary.GetObjectName` (`RitualPosition.OccupyingCharacter` _as_ritual_position))))))))))

(fn `CheckIsOccupied`
  (returns (ReturnValue :type Boolean))
  (return (`RitualPosition.IsOccupied` (`self.As Ritual Position`))))

(fn `GetCharacter`
  (params (Object :type "Object Object Reference"))
  (returns (Output_Get :type "/Game/Blueprints/Character/BP_WitchPTCharacter Object Reference"))
  (bind _asbp_witch_ptcharacter (cast `/Game/Blueprints/Character/BP_WitchPTCharacter` Object)
    (:`then`
      (bind _output_get (set `self.As BP Witch PTCharacter` _asbp_witch_ptcharacter)))
    (:`CastFailed`
      _))
  (return _output_get))

(fn `GetRitualPositionObject`
  (params (Object :type "Object Object Reference"))
  (bind _asbp_ritual_position (cast `/Game/Blueprints/Item/Ritual/BP_Ritual_Position` Object))
  (set `self.As Ritual Position` _asbp_ritual_position))