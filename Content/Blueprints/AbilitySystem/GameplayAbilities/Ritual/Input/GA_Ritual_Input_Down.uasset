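; Gameplay ability for the "Down" ritual input of a witch player interacting with a ritual altar.
; On activation it binds to the altar's input-received event and sends its input tag to the altar's server input handler.
; The result picks a montage: a table stab for a correct input at Ritual.Position.1, none assigned for other positions, a stagger knockdown when wrong.
; The ability ends after a short delay.
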(event `self.K2_ActivateAbility`
  (`|ExecutionSequence`
    (:`then_0`
      (bind _aswitch_ptcharacter (cast `WitchPTCharacter` (`self.GetAvatarActorFromActorInfo`)))
      (bind _asbp_witch_ptplayer_state (cast `/Game/Blueprints/Player/BP_WitchPTPlayerState` (`Pawn.PlayerState` _aswitch_ptcharacter))))
    (:`then_1`
      (bind _ritualaltarinteractingwith (`WitchPTPlayerState.RitualAltarInteractingWith` _asbp_witch_ptplayer_state))
      (add `RitualAltar.OnInputReceived` _ritualaltarinteractingwith (delegate `OnInputReceived_Event`)))
    (:`then_2`
      (`RitualAltar.Server_HandlePlayerInput` _ritualaltarinteractingwith _aswitch_ptcharacter (`self.Input Tag`)))))

(event `OnInputReceived_Event`
  (params (ReceivedTag :type "GameplayTag Structure (by ref)") (bWasCorrect :type Boolean))
  (if bWasCorrect
    (if (`BlueprintGameplayTagLibrary.MatchesTag` (`RitualPosition.GetPositionTag` (`WitchPTPlayerState.RitualPositionInteractingWith` (stale `self.K2_ActivateAbility` _asbp_witch_ptplayer_state))) (struct :`TagName` "Ritual.Position.1") true)
      (`AbilityTask_PlayMontageAndWait.CreatePlayMontageAndWaitProxy` "None" "/Game/WitchHag/WitchHag_Paired_Stab_OnTable_Attacker_Montage.WitchHag_Paired_Stab_OnTable_Attacker_Montage" 1.0 "None" false
        (:`then`
          _))
      (else
        (`AbilityTask_PlayMontageAndWait.CreatePlayMontageAndWaitProxy` "None" null 1.0 "None" false
          (:`then`
            _))))
    (else
      (`AbilityTask_PlayMontageAndWait.CreatePlayMontageAndWaitProxy` "None" "/Game/BattleWitch/AnimSequence/UE5/Anim_BattleWitchStaggerKnockDown_Montage.Anim_BattleWitchStaggerKnockDown_Montage" 1.0 "None" false
        (:`then`
          _))))
  (`GameplayTask_WaitDelay.TaskWaitDelay` null 1.0
    (:`OnFinish`
      (`self.K2_EndAbility`))))