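; Gameplay ability for the left input in the ritual, sending the player's input to the ritual and playing the resulting animation.
; On activation it binds to the altar of the avatar's ritual position, then passes its input tag through RitualInterface.
; The altar's response selects a montage: stab at position 1 or left turn elsewhere when correct, knockdown when wrong.
; The ability ends shortly after the montage starts, leaving it playing.
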(event `self.K2_ActivateAbility`
  (bind _returnvalue (`self.GetAvatarActorFromActorInfo`))
  (if (`KismetSystemLibrary.DoesImplementInterface` _returnvalue "/Script/WitchPT.RitualInterface")
    (bind _output_get (set `self.AvatarActor` _returnvalue))
    (bind _ascharacter (cast `Character` _output_get))
    (bind _returnvalue_2 (message `RitualInterface.GetRitualPosition` (`self.AvatarActor`)))
    (set `self.AltarPosition` _returnvalue_2)
    (add `RitualAltar.OnInputReceived` (`RitualPosition.GetRitualAltar` _returnvalue_2) (delegate `OnInputReceived_Event`))
    (message `RitualInterface.HandlePlayerInput` (`self.AvatarActor`) _ascharacter (`self.Input Tag`))))

(event `OnInputReceived_Event`
  (params (ReceivedTag :type "GameplayTag Structure (by ref)") (bWasCorrect :type Boolean))
  (if bWasCorrect
    (if (and bWasCorrect (`BlueprintGameplayTagLibrary.MatchesTag` (`RitualPosition.GetPositionTag` (`self.AltarPosition`)) (struct :`TagName` "Ritual.Position.1") true))
      (`AbilityTask_PlayMontageAndWait.CreatePlayMontageAndWaitProxy` "None" "/Game/WitchHag/WitchHag_Paired_Stab_OnTable_Attacker_Montage.WitchHag_Paired_Stab_OnTable_Attacker_Montage" 2.0 "None" false
        (:`then`
          _))
      (else
        (`AbilityTask_PlayMontageAndWait.CreatePlayMontageAndWaitProxy` "None" "/Game/BattleWitch/AnimSequence/UE5/Anim_BattleWitchTurnLeft90_Montage.Anim_BattleWitchTurnLeft90_Montage" 1.0 "None" false
          (:`then`
            _))))
    (else
      (`AbilityTask_PlayMontageAndWait.CreatePlayMontageAndWaitProxy` "None" "/Game/BattleWitch/AnimSequence/UE5/Anim_BattleWitchStaggerKnockDown_Montage.Anim_BattleWitchStaggerKnockDown_Montage" 1.0 "None" false
        (:`then`
          _))))
  (`AbilityTask_WaitDelay.WaitDelay` 0.5
    (:`OnFinish`
      (`self.K2_EndAbility`))))