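; Gameplay ability that collects the item the avatar is currently interacting with into the player's inventory.
; On activation it caches player controller 0's inventory component and the avatar's interaction component, then passes the current interactable's BP_Inv_InventoryItem component to TryAddItem.
; The live path never calls EndAbility.
; An alternative authority-checked pickup with gameplay cue and actor removal, plus a delayed end, sit disconnected.
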(event `self.K2_ActivateAbility`
  (bind _returnvalue (`Int_InteractionSystemComponent.GetInteractionSystemComponent` (`self.GetAvatarActorFromActorInfo`)))
  (bind _returnvalue_2 (`Actor.GetComponentByClass` (`Int_InteractionSystemComponent.CurrentInteractableActor` (`self.Interaction Component`)) "/AndresD3v_InventorySystem/Items/BP_Inv_InventoryItem.BP_Inv_InventoryItem_C"))
  (`|ExecutionSequence`
    (:`then_0`
      (bind _returnvalue_3 (`Inv_InventoryStatics.GetInventoryComponent` (`GameplayStatics.GetPlayerController` 0)))
      (set `self.Inventory_Component` _returnvalue_3))
    (:`then_1`
      (`/Engine/EditorBlueprintResources/StandardMacros.IsValid` _returnvalue
        (:`Is Valid`
          (set `self.Interaction Component` _returnvalue))))
    (:`then_2`
      (`/Engine/EditorBlueprintResources/StandardMacros.IsValid` _returnvalue_2
        (:`Is Valid`
          (`Inv_InventoryComponent.TryAddItem` (`self.Inventory_Component`) _returnvalue_2))))))