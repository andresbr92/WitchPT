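; Gameplay ability that tells a tap from a hold on interaction input and broadcasts the result as an async message.
; Input press starts a looping timer that increments a counter up to MaxTime.
; Reaching MaxTime broadcasts HoldActivate and ends the ability after a short delay.
; Input release ends the ability, broadcasts Activate if the counter is below MaxTime, then resets the counter.
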(event `self.K2_ActivateAbility`
  (`|ExecutionSequence`
    (:`then_0`
      (`AbilityTask_WaitInputPress.WaitInputPress` false
        (:`OnPress`
          (`KismetSystemLibrary.K2_SetTimerDelegate` (delegate `CustomEvent`) 0.01 true))))
    (:`then_1`
      (`AbilityTask_WaitInputRelease.WaitInputRelease` false
        (:`OnRelease`
          (`self.K2_EndAbility`)
          (if (< (`self.Time`) (`self.MaxTime`))
            (`AsyncMessageSystemBlueprintLibrary.QueueAsyncMessageForBroadcast` (make `AsyncMessageId` (struct :`TagName` "Ability.Interaction.Activate"))))
          (set `self.Time` 0))))))

(event `CustomEvent`
  (if (< (`self.Time`) (`self.MaxTime`))
    (set `self.Time` (+ (`self.Time`) 1))
    (if (== (`self.Time`) (`self.MaxTime`))
      (`AsyncMessageSystemBlueprintLibrary.QueueAsyncMessageForBroadcast` (make `AsyncMessageId` (struct :`TagName` "Ability.Interaction.HoldActivate")))
      (`GameplayTask_WaitDelay.TaskWaitDelay` null 0.2
        (:`OnFinish`
          (`self.K2_EndAbility`))))))