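; GA_Aim is a gameplay ability that puts the WitchPT character into aim mode while its input is held.
; On activation it applies the GE_StandardAim effect to the owner, calls StartAim on the character and waits for input release.
; Releasing the input ends the ability, which removes the stored effect by handle and calls StopAim.
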(event `self.K2_ActivateAbility`
  (bind _asbp_witch_ptcharacter (cast `/Game/Blueprints/Character/BP_WitchPTCharacter` (`self.GetAvatarActorFromActorInfo`)))
  (set `self.As BP Witch PTCharacter` _asbp_witch_ptcharacter)
  (bind _returnvalue (`self.BP_ApplyGameplayEffectToOwner` "/Game/Blueprints/AbilitySystem/GameplayAbilities/Aim/GE_StandardAim.GE_StandardAim_C"))
  (set `self.GEAim` _returnvalue)
  (`/Game/Blueprints/Character/BP_WitchPTCharacter.StartAim` (`self.As BP Witch PTCharacter`))
  (`AbilityTask_WaitInputRelease.WaitInputRelease` false
    (:`OnRelease`
      (`self.K2_EndAbility`))))

(event `self.K2_OnEndAbility`
  (params (bWasCancelled :type Boolean))
  (`self.BP_RemoveGameplayEffectFromOwnerWithHandle` (`self.GEAim`))
  (`/Game/Blueprints/Character/BP_WitchPTCharacter.StopAim` (`self.As BP Witch PTCharacter`)))