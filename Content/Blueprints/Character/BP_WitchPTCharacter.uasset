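; Witch player character with aim camera zoom and cauldron interaction.
; Start and stop aim events drive spring arm length through timelines.
; Each tick a debug-drawn sphere overlap feeds nearby cauldron actors to the interaction system, and F makes the first one current.
; Key 0 chains server-only and client-only events that swap the mesh material to a laser pointer one; smart object slot claiming and role display are disconnected.
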(event `StartAim`
  (bind (_direction _armlength) (`Timeline|Timeline_Start_Aim` :!via `PlayFromStart`)
    (:`Update`
      (set `SpringArmComponent.TargetArmLength` _armlength (`self.SpringArm`)))))

(event `StopAim`
  (bind (_direction _armlength) (`Timeline|Timeline` :!via `PlayFromStart`)
    (:`Update`
      (set `SpringArmComponent.TargetArmLength` _armlength (`self.SpringArm`)))))

(event `self.ReceiveBeginPlay`)

(event `self.ReceiveTick`
  (params (DeltaSeconds :type "Float (single-precision)"))
  (`KismetSystemLibrary.DrawDebugSphere` (`self.K2_GetActorLocation`) 200.0)
  (bind _outactors (`KismetSystemLibrary.SphereOverlapActors` (`self.K2_GetActorLocation`) 200.0 (`self.Object Types`) "/Game/Blueprints/SmartObjects/BP_SO_Cauldron.BP_SO_Cauldron_C"))
  (`Int_InteractionSystemComponent.SetInteractableActors` (`self.Int_InteractionSystem`) _outactors))

(event `Key|F`
  (params (Key :type "Key Structure"))
  (bind _int_interactionsystem (`self.Int_InteractionSystem`))
  (bind _interactableactors (`Int_InteractionSystemComponent.InteractableActors` _int_interactionsystem))
  (:`Pressed`
    (if (`KismetArrayLibrary.Array_IsValidIndex` _interactableactors)
      (`Int_InteractionSystemComponent.SetCurrentInteractableActor` _int_interactionsystem (`|GetArrayItem` _interactableactors)))))

(event `Key|Zero`
  (params (Key :type "Key Structure"))
  (:`Pressed`
    (`self.Server_Only`)))

(event `Server_Only`
  (`PrimitiveComponent.SetMaterial` (`self.Mesh`) 0 "/Engine/VREditor/LaserPointer/LaserPointerMaterial.LaserPointerMaterial")
  (`PrimitiveComponent.SetMaterial` (`self.Mesh`) 0 "/Engine/VREditor/LaserPointer/LaserPointerMaterial.LaserPointerMaterial")
  (`self.Client_Only`))

(event `Client_Only`
  (`PrimitiveComponent.SetMaterial` (`self.Mesh`) 0 "/Engine/VREditor/LaserPointer/LaserPointerMaterial.LaserPointerMaterial"))

(fn `UserConstructionScript`)