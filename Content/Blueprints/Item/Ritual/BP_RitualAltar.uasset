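; Ritual altar actor that sets up the four ritual positions around itself when play begins.
; It gathers four spawn-point components, caches the witch game mode, then spawns a ritual position actor at each point's world transform.
; Each spawned actor receives a tag matched by index and a reference back to the altar.
; Player-count-based point selection and tracking of spawned positions are left disconnected.
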(event `self.ReceiveBeginPlay`
  (`KismetArrayLibrary.Array_Add` (`self.PositionSpawnPoints`) (`self.SpawnPoint_Position_1`))
  (`KismetArrayLibrary.Array_Add` (`self.PositionSpawnPoints`) (`self.SpawnPoint_Position_2`))
  (`KismetArrayLibrary.Array_Add` (`self.PositionSpawnPoints`) (`self.SpawnPoint_Position_3`))
  (`KismetArrayLibrary.Array_Add` (`self.PositionSpawnPoints`) (`self.SpawnPoint_Position_4`))
  (bind _asbp_witch_game_mode (cast `/Game/Blueprints/Game/BP_WitchGameMode` (`GameplayStatics.GetGameMode`)))
  (set `self.As BP Witch Game Mode` _asbp_witch_game_mode)
  (`|ExecutionSequence`
    (:`then_0`
      (for (_array_element _array_index) (`self.PositionSpawnPoints`)
        (bind _returnvalue (`|SpawnActorFromClass` (`self.RitualPositionClass`) (`SceneComponent.K2_GetComponentToWorld` _array_element) "AlwaysSpawn" "MultiplyWithRoot" null null))
        (`|ExecutionSequence`
          (:`then_0`
            (`RitualPosition.SetPositionTag` _returnvalue (`|GetArrayItem` (`self.TagsPositions`) _array_index)))
          (:`then_1`
            (`RitualPosition.SetRitualAltar` _returnvalue self)))))))

(event `self.ReceiveTick`
  (params (DeltaSeconds :type "Float (single-precision)")))

(fn `UserConstructionScript`)